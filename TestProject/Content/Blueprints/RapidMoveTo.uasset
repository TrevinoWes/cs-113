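; RapidMoveTo is a behavior tree task that sends a mob pawn toward the blackboard's TargetToFollow actor.
; It caches the mob_AIController on first execution, then runs AIMoveTo to the target's X and Y at the pawn's own Z.
; It finishes successfully as soon as the move is issued, as well as on move success, so the tree does not wait for arrival.
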(event `self.ReceiveExecute`
  (params (OwnerActor :type "Actor Object Reference"))
  (bind _returnvalue (`Controller.K2_GetPawn` (`self.AI_CON_ref`)))
  (if (not (!= (`self.AI_CON_ref`) null))
    (bind _asmob_aicontroller (cast `/Game/Blueprints/mob_AIController` OwnerActor))
    (set `self.AI_CON_ref` _asmob_aicontroller))
  (`|AIMoveTo` _returnvalue (`KismetMathLibrary.MakeVector` (.x (`Actor.K2_GetActorLocation` (`BTFunctionLibrary.GetBlackboardValueAsActor` (`self.target_to_follow`)))) (.y (`Actor.K2_GetActorLocation` (`BTFunctionLibrary.GetBlackboardValueAsActor` (`self.target_to_follow`)))) (.z (`Actor.K2_GetActorLocation` _returnvalue))) null 50.0
    (:`then`
      _)
    (:`OnSuccess`
      _))
  (`self.FinishExecute` true))