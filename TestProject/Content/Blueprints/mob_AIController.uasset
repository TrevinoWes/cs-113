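; AI controller for mobs that sets up their blackboard and behavior tree to target a player.
; On BeginPlay it loads Mob_board, gets all PlayerBase_Blueprint actors and takes the first one found.
; It writes that actor to TargetToFollow and its current location to TargetLocation, then runs Mob_tree.
; The target location is captured only once, and the tree never starts if no player actor exists at that moment.
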(event `self.ReceiveBeginPlay`
  (bind _returnvalue (`AIBlueprintHelperLibrary.GetBlackboard` self))
  (`self.UseBlackboard` "/Game/Blueprints/mob_board.mob_board")
  (bind _outactors (`GameplayStatics.GetAllActorsOfClass` "/Game/Blueprints/PlayerBase_Blueprint.PlayerBase_Blueprint_C"))
  (for (_array_element _array_index) _outactors
    (if (== _array_index 0)
      (`BlackboardComponent.SetValueAsObject` _returnvalue (`self.target_to_follow`) _array_element)
      (`BlackboardComponent.SetValueAsVector` _returnvalue (`self.TargetLocation`) (`self.K2_GetActorLocation` _array_element))
      (`self.RunBehaviorTree` "/Game/Blueprints/mob_tree.mob_tree"))))

(fn `UserConstructionScript`)