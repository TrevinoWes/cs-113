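; Tower actor that automatically acquires and attacks Character_Blueprint actors within range.
; Each Tick, it scans all such actors for the first in range when it has no valid target, or drops its current target once out of range.
; Acquiring a target starts a Delay-driven Attack loop paced by Speed that runs while Attacking is set.
; The attack only prints debug text; Damage, initialized in the Construction Script, is never applied.
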(event `Attack`
  (`KismetSystemLibrary.PrintString` "Attack" :!label _label)
  (`KismetSystemLibrary.Delay` (`self.Speed`))
  (if (`self.attacking`)
    (goto _label)))

(event `self.ReceiveTick`
  (params (DeltaSeconds :type "Float (single-precision)"))
  (`/Engine/EditorBlueprintResources/StandardMacros.IsValid` (`self.monsterTarget`)
    (:`Is Valid`
      (if (> (`KismetMathLibrary.VSize` (- (`self.K2_GetActorLocation` (`self.monsterTarget`)) (`self.K2_GetActorLocation`))) (`self.Range`))
        (set `self.monsterTarget` null)
        (set `self.attacking` false)
        (`KismetSystemLibrary.PrintString` "Stop Attacking")))
    (:`Is Not Valid`
      (bind _outactors (`GameplayStatics.GetAllActorsOfClass` "/Game/Blueprints/Character_Blueprint.Character_Blueprint_C"))
      (for _array_element _outactors
        (if (<= (`KismetMathLibrary.VSize` (- (`self.K2_GetActorLocation` _array_element) (`self.K2_GetActorLocation`))) (`self.Range`))
          (set `self.monsterTarget` _array_element)
          (`KismetSystemLibrary.PrintString` "Start Attacking")
          (set `self.attacking` true)
          (`self.Attack`)
          (break))))))

(fn `UserConstructionScript`
  (set `self.Damage` 10.0)
  (set `self.Speed` 1.0)
  (set `self.Range` 850.0))